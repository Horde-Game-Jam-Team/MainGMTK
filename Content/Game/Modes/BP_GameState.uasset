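; Game state Blueprint that tracks the speed of a spinning wheel and sends it to the first-person player controller for display.
; BeginWheelSpin sets the minimum speed and starts Tick accumulating time.
; Tick recomputes speed through a passive-increase function built around logarithmic growth above that minimum.
; IncreaseWheelSpeed calls a placeholder calculation that ignores the increase amount, and Tick overwrites its result while spinning.
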(event `BeginWheelSpin`
  (params (Speed :type "Float (double-precision)"))
  (set `self.Minimum Wheel Speed` Speed)
  (set `self.IsWheelSpinning` true))

(event `Increase Wheel Speed`
  (params (`Event Increase amount` :type "Float (double-precision)"))
  (set `self.WheelSpeed` (`self.UNIMPLEMENTED Wheel Speed Increase Event Calculation` (`self.WheelSpeed`) `Event Increase amount`)))

(event `self.ReceiveTick`
  (params (DeltaSeconds :type "Float (single-precision)"))
  (if (`self.IsWheelSpinning`)
    (bind _output_get (set `self.Elapsed time` (+ DeltaSeconds (`self.Elapsed time`))))
    (bind _output_get_2 (set `self.WheelSpeed` (`self.Passive Wheel Speed Increase` _output_get 1.0 (`self.Minimum Wheel Speed`))))
    (bind _asbp_first_person_player_controller (cast `/Game/Game/Characters/Player/BP_FirstPersonPlayerController` (`GameplayStatics.GetPlayerController` 0)))
    (`/Game/Game/Characters/Player/BP_FirstPersonPlayerController.Event UpdateWheelSpeedDisplay` _asbp_first_person_player_controller _output_get_2)))

(fn `UserConstructionScript`)