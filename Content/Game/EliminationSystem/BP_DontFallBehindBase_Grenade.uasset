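; Grenade actor in the DontFallBehind elimination system that flies at the player and takes them out.
; On BeginPlay it jumps to a point behind on world X and high above the player, then a timeline lerps it toward the player's live position.
; The sine arc height term has a constant zero input, so it adds no arc.
; When the timeline finishes, it disables player input and ragdolls the mesh through physics simulation.
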(event `self.ReceiveBeginPlay`
  (bind _returnvalue (+ (`self.K2_GetActorLocation` (`self.Player`)) (-500.0 0.0 2000.0)))
  (`parent.ReceiveBeginPlay`)
  (`self.K2_SetActorLocation` _returnvalue)
  (set `self.Startlocation` _returnvalue)
  (bind (_direction _time) (`Timeline|ParabolicMove` :!via `PlayFromStart`)
    (:`Update`
      (`self.K2_SetActorLocation` (`KismetMathLibrary.MakeVector` (.x (`KismetMathLibrary.VLerp` (`self.StartLocation`) (`self.K2_GetActorLocation` (`self.Player`)) _time)) (.y (`KismetMathLibrary.VLerp` (`self.StartLocation`) (`self.K2_GetActorLocation` (`self.Player`)) _time)) (+ (.z (`KismetMathLibrary.VLerp` (`self.StartLocation`) (`self.K2_GetActorLocation` (`self.Player`)) _time)) (* (`KismetMathLibrary.Sin` (* 0.0 (`KismetMathLibrary.GetPI`))) (`self.ArcHeight`))))))
    (:`Finished`
      (`self.Finish`))))

(event `Finish`
  (bind _player (`self.Player`))
  (`self.DisableInput` _player (`GameplayStatics.GetPlayerController` 0))
  (`PrimitiveComponent.SetSimulatePhysics` (`Character.Mesh` _player) true))

(fn `UserConstructionScript`
  (`parent.UserConstructionScript`))