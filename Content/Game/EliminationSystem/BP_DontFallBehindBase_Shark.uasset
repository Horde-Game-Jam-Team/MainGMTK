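; Shark elimination effect, a child of a DontFallBehind base, in which a shark rises from beneath the player.
; On BeginPlay it moves below the player and blends the view to a newly spawned offset camera aimed at them.
; A timeline lerps the mesh upward while a short parallel delay triggers a Niagara debris burst and hides the player's mesh, selling the hit.
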(event `self.ReceiveBeginPlay`
  (bind _player (`self.Player`))
  (bind _staticmesh (`self.StaticMesh`))
  (bind _returnvalue (`self.K2_GetActorLocation` (`self.Player`)))
  (bind _returnvalue_2 (+ _returnvalue (1000.0 1000.0 1500.0)))
  (`parent.ReceiveBeginPlay`)
  (`self.K2_SetActorLocation` (- (`self.K2_GetActorLocation` (`self.Player`)) (0.0 0.0 500.0)))
  (bind _returnvalue_3 (`|SpawnActorFromClass` "/Script/Engine.CameraActor" (`KismetMathLibrary.MakeTransform` _returnvalue_2 (`KismetMathLibrary.FindLookAtRotation` _returnvalue_2 _returnvalue)) "Undefined" "MultiplyWithRoot" null null))
  (`PlayerController.SetViewTargetWithBlend` (`GameplayStatics.GetPlayerController` 0) _returnvalue_3 0.2 "VTBlend_Linear" 0.0 false)
  (bind _output_get (set `self.StartLocation` (`SceneComponent.RelativeLocation` _staticmesh)))
  (set `self.EndLocation` (+ _output_get (0.0 0.0 1300.0)))
  (`|ExecutionSequence`
    (:`then_0`
      (bind (_direction _alpha) (`Timeline|SharkTimeline` :!via `PlayFromStart`)
        (:`Update`
          (`SceneComponent.K2_SetRelativeLocation` _staticmesh (`KismetMathLibrary.VLerp` (`self.StartLocation`) (`self.EndLocation`) _alpha) false false))))
    (:`then_1`
      (`KismetSystemLibrary.Delay` 0.4)
      (`NiagaraFunctionLibrary.SpawnSystemAtLocation` "/Game/Game/Library/Niagara/NiagaraSystems/NS_ExplosionDebris.NS_ExplosionDebris" (`self.K2_GetActorLocation` _player))
      (`SceneComponent.SetVisibility` (`Character.Mesh` _player) false false))))

(fn `UserConstructionScript`
  (`parent.UserConstructionScript`))