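; BPC_DontFallBehind is an elimination-system component on BP_FirstPersonCharacter that punishes the player for falling behind.
; On BeginPlay it caches the owning character and binds to its OnFallBehindPunish dispatcher.
; ActivateFallBehindPunish picks a random class from the Mechanics array and spawns it at the player's location, passing in the player reference.
; The component does not detect falling behind itself; it only supplies the punishment.
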(event `self.ReceiveBeginPlay`
  (bind _asbp_first_person_character_ (cast `/Game/Game/Characters/Player/BP_FirstPersonCharacter` (`self.GetOwner`)))
  (bind _output_get (set `self.Player` _asbp_first_person_character_))
  (add `RPGCharacter.OnFallBehindPunish` _output_get (`|CreateDelegate` :!event `ActivateFallBehindPunish`)))

(event `ActivateFallBehindPunish`
  (bind _player (`self.Player`))
  (`|SpawnActorFromClass` (`KismetArrayLibrary.Array_Random` (`self.Mechanics`)) (`KismetMathLibrary.MakeTransform` (`Actor.K2_GetActorLocation` _player)) "AdjustIfPossibleButAlwaysSpawn" "MultiplyWithRoot" null _player null))