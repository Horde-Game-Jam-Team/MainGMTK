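; Generic RPG character Blueprint with a fireball attack, damage handling and a point light that follows it.
; Pressing Z fires through the BPFireball component.
; Any damage taken goes to BPStatusComponent and triggers a world camera shake at the character.
; Each tick, FireFollow targets a point trailing the Cube against velocity, or the Cube itself when nearly still, and updates the light's position through SetCurrentLightPosition.
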(event `OnTakeAnyDamage_Event` :!signature `self.OnTakeAnyDamage`
  (params (DamagedActor :type "Actor Object Reference") (Damage :type "Float (single-precision)") (DamageType :type "DamageType Object Reference") (InstigatedBy :type "Controller Object Reference") (DamageCauser :type "Actor Object Reference"))
  (`StatusComponent.TakeDamage` (`self.BP_StatusComponent`) (`KismetMathLibrary.FTrunc` Damage))
  (`GameplayStatics.PlayWorldCameraShake` "/Game/Game/Characters/Player/LCS_CameraShake.LCS_CameraShake_C" (`self.K2_GetActorLocation`) 0.0 500.0))

(event `self.ReceiveBeginPlay`
  (add `self.OnTakeAnyDamage` (delegate `OnTakeAnyDamage_Event`))
  (set `self.CurrentLightLocation` (`SceneComponent.K2_GetComponentLocation` (`self.Cube`))))

(event `self.ReceiveTick`
  (params (DeltaSeconds :type "Float (single-precision)"))
  (`self.FireFollow` DeltaSeconds) ; Can replace the point light with anything.
)

(event `Key|Z`
  (params (Key :type "Key Structure"))
  (:`Pressed`
    (`self.Aim`)))

(fn `Aim`
  (locals (Start :type "Vector Structure") (`Forward Vector` :type "Vector Structure" :default (0.0 0.0 0.0)) (End :type "Vector Structure"))
  (`/Game/Game/Characters/Player/BP_Fireball.Shoot` (`self.BP_Fireball`)))

(fn `FireFollow`
  (params (DeltaTime :type "Float (single-precision)"))
  (locals (Delta :type "Float (single-precision)") (Velocity :type "Vector Structure") (TargetLocation :type "Vector Structure"))
  (set `local.Delta` DeltaTime)
  (set `local.Velocity` (`self.GetVelocity`))
  (if (> (`KismetMathLibrary.VSize` (`local.Velocity`)) 5.0)
    (set `local.TargetLocation` (- (`SceneComponent.K2_GetComponentLocation` (`self.Cube`)) (* (`KismetMathLibrary.Normal` (`local.Velocity`)) (`self.MaxOffset`))))
    (else
      (set `local.TargetLocation` (`SceneComponent.K2_GetComponentLocation` (`self.Cube`)))))
  (bind _output_get (set `self.CurrentLightLocation` (`KismetMathLibrary.VInterpTo` (`self.CurrentLightLocation`) (`local.TargetLocation`) (`local.Delta`) (`self.InterpSpeed`))))
  (`SceneComponent.K2_SetWorldLocation` (`self.Point Light`) _output_get false false))

(fn `UserConstructionScript`)