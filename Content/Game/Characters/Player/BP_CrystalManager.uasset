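; BP_CrystalManager tracks the player's crystal count as a spendable resource.
; CollectCrystal and SpendCrystal add or subtract an amount, clamping the result between zero and MaxCrystals.
; CanSpendCrystal reports whether the count covers a given amount, but SpendCrystal does not check it itself, so an overspend simply clamps to zero.
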(fn `CanSpendCrystal`
  (params (Amount :type Integer))
  (returns (ReturnValue :type Boolean))
  (return (>= (`self.Crystals`) Amount)))

(fn `Collect Crystal`
  (params (Amount :type Integer))
  (set `self.Crystals` (`KismetMathLibrary.Clamp` (+ (`self.Crystals`) Amount) 0 (`self.MaxCrystals`))))

(fn `SpendCrystal`
  (params (Amount :type Integer))
  (set `self.Crystals` (`KismetMathLibrary.Clamp` (- (`self.Crystals`) Amount) 0 (`self.MaxCrystals`))))