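; BP_GrapplingHook is the player's hook shot, tracing forward from the owner's camera and returning the actor it hits.
; Shoot takes a short-range visibility line trace from Set Positions, ignores the owner, then branches through Hit or Miss.
; Each branch calls SpawnSpark with its own fire emitter and a shared fireball sound.
; No pulling logic is present, and SpawnBomb's actor spawn is left unconnected.
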(fn `Shoot`
  (returns (HitActor :type "Actor Object Reference"))
  (locals (Start :type "Vector Structure" :default (0.0 0.0 0.0)) (End :type "Vector Structure") (ForwardVector :type "Vector Structure") (LaunchVelocity :type "Float (double-precision)" :default 1000.0) (CrystalManager :type "/Game/Game/Characters/Player/BP_CrystalManager Object Reference"))
  (bind _returnvalue (`Actor.GetComponentByClass` (`self.GetOwner`) "/Script/Engine.CameraComponent"))
  (set `local.Start` (`SceneComponent.K2_GetComponentLocation` _returnvalue))
  (set `local.ForwardVector` (`SceneComponent.GetForwardVector` _returnvalue))
  (set `local.End` (+ (`local.Start`) (* (`local.ForwardVector`) 1000.0)))
  (bind (_outhit _returnvalue_2) (`KismetSystemLibrary.LineTraceSingle` (`local.Start`) (`local.End`) "TraceTypeQuery1" false (`|MakeArray` (`self.GetOwner`)) "ForDuration"))
  (if _returnvalue_2
    (bind (_bblockinghit _binitialoverlap _time _distance _location _impactpoint _normal _impactnormal _physmat _hitactor) (`GameplayStatics.BreakHitResult` _outhit))
    (`self.SpawnSpark` "/Game/M5VFXVOL2/Particles/Explosion/Fire_Exp_00.Fire_Exp_00" _impactpoint)
    (return _hitactor)
    (else
      (`self.SpawnSpark` "/Game/M5VFXVOL2/Particles/Explosion/Fire_Exp_04.Fire_Exp_04" (`KismetMathLibrary.SelectVector` _impactpoint (`local.End`) _returnvalue_2)))))

(fn `SpawnBomb`
  (params (Location :type "Vector Structure")))

(fn `SpawnSpark`
  (params (EmitterTemplate :type "ParticleSystem Object Reference") (Location :type "Vector Structure"))
  (`GameplayStatics.SpawnEmitterAtLocation` EmitterTemplate Location)
  (`GameplayStatics.PlaySound2D` "/Game/Sounds/Fireball/LOL_SFX_Fireball_Large_1.LOL_SFX_Fireball_Large_1" 1.0 1.0 0.0 null null))