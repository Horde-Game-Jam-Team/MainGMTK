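; Generic AI enemy character Blueprint that detects the player, attacks, takes damage and drops an item when destroyed.
; AI perception of an RPGCharacter sets the SeesPlayer blackboard key, and AttackPlayer plays a montage, locking CanAttack for its duration.
; Hit-sphere contact damages RPGCharacters while CanAttack is true.
; Bound delegates route incoming damage to StatusComponent and destruction to ItemDropComponent; an older launch-based charge attack remains.
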(event `OnTakeAnyDamage_Event` :!signature `self.OnTakeAnyDamage`
  (params (DamagedActor :type "Actor Object Reference") (Damage :type "Float (single-precision)") (DamageType :type "DamageType Object Reference") (InstigatedBy :type "Controller Object Reference") (DamageCauser :type "Actor Object Reference"))
  (`StatusComponent.TakeDamage` (`self.Status Component`) (`KismetMathLibrary.FTrunc` Damage)))

(event `OnDestroyed_Event` :!signature `self.OnDestroyed`
  (params (DestroyedActor :type "Actor Object Reference"))
  (`ItemDropComponent.SpawnItem` (`self.Item Drop Component`)))

(event `self.ReceiveBeginPlay`
  (add `self.OnTakeAnyDamage` (delegate `OnTakeAnyDamage_Event`))
  (add `self.OnDestroyed` (delegate `OnDestroyed_Event`))
  (bind _returnvalue (`self.PlayAnimMontage` "/Game/Game/Library/Mannequins/Anims/Pistol/MM_Pistol_Fire_Montage.MM_Pistol_Fire_Montage"))
  (`KismetSystemLibrary.Delay` _returnvalue)
  (`KismetSystemLibrary.PrintText` "Hello"))

(event `self.AIPerception.OnTargetPerceptionUpdated`
  (params (Actor :type "Actor Object Reference") (Stimulus :type "AIStimulus Structure"))
  (bind (_returnvalue _key_name) (`self.GetBlackboard` "SeesPlayer"))
  (bind _asrpgcharacter (cast `RPGCharacter` Actor))
  (`AIPerceptionComponent.GetActorsPerception` (`self.AIPerception`) self)
  (`BlackboardComponent.SetValueAsBool` _returnvalue _key_name true)
  (`KismetSystemLibrary.PrintText` (`|FormatText` "{Owner}: I notice you {Player}!" self _asrpgcharacter)))

(event `self.Damage Hit Sphere.OnComponentHit`
  (params (HitComponent :type "PrimitiveComponent Object Reference") (OtherActor :type "Actor Object Reference") (OtherComp :type "PrimitiveComponent Object Reference") (NormalImpulse :type "Vector Structure") (Hit :type "HitResult Structure (by ref)"))
  (if (`self.CanAttack`)
    (bind _asrpgcharacter (cast `RPGCharacter` OtherActor))
    (`GameplayStatics.ApplyDamage` _asrpgcharacter 2.0)))

(event `Attack Player`
  (if (`self.CanAttack`)
    (`self.Attack Event`)
    (set `self.CanAttack` false)))

(event `Attack Event`
  (bind _returnvalue (`self.PlayAnimMontage` "/Game/Game/Library/Mannequins/Anims/Pistol/MM_Pistol_Fire_Montage.MM_Pistol_Fire_Montage"))
  (`KismetSystemLibrary.Delay` _returnvalue)
  (set `self.CanAttack` true))

(fn `Attack Player (OLD)`
  (bind (_returnvalue _key_name) (`self.GetBlackboard` "IsCharging"))
  (`self.LaunchCharacter` (* (`KismetMathLibrary.Normal` (- (`self.K2_GetActorLocation` (`GameplayStatics.GetPlayerCharacter` 0)) (`self.K2_GetActorLocation`))) (`self.Charge Speed`)) true true)
  (`BlackboardComponent.SetValueAsBool` _returnvalue _key_name false))

(fn `GetBlackboard`
  (params (Value :type Name))
  (returns (ReturnValue :type "BlackboardComponent Object Reference") (`Key Name` :type Name))
  (return (`AIBlueprintHelperLibrary.GetBlackboard` (`AIBlueprintHelperLibrary.GetAIController` self)) (`KismetSystemLibrary.MakeLiteralName` Value)))

(fn `UserConstructionScript`)