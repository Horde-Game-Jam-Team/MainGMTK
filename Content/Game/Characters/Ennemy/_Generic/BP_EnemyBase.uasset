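; Base enemy character that can switch between walking and running, attack RPG characters, take damage and drop loot.
; Attack plays a montage with the sphere hitbox enabled, applies fixed damage once per swing via a hit flag, then signals whether the attack completed or was interrupted.
; BeginPlay binds incoming damage to the status component and destruction to the item drop component, which spawns an item.
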(event `OnTakeAnyDamage_Event` :!signature `self.OnTakeAnyDamage`
  (params (DamagedActor :type "Actor Object Reference") (Damage :type "Float (single-precision)") (DamageType :type "DamageType Object Reference") (InstigatedBy :type "Controller Object Reference") (DamageCauser :type "Actor Object Reference"))
  (`StatusComponent.TakeDamage` (`self.BP_StatusComponentEnemy`) (`KismetMathLibrary.FTrunc` Damage)))

(event `OnDestroyed_Event` :!signature `self.OnDestroyed`
  (params (DestroyedActor :type "Actor Object Reference"))
  (`ItemDropComponent.SpawnItem` (`self.Item Drop Component`))
  (`KismetSystemLibrary.PrintText` "ENEMY IS DEFEATED"))

(event `self.ReceiveBeginPlay`
  (add `self.OnTakeAnyDamage` (delegate `OnTakeAnyDamage_Event`))
  (add `self.OnDestroyed` (delegate `OnDestroyed_Event`)))

(event `/Game/Game/Characters/Ennemy/AI/BPI_EnemyAI.SetMovementSpeed`
  (params (NewEnemyMovSpeed :type "/Game/Game/Characters/Ennemy/AI/E_MovementSpeed Enum" :default "NewEnumerator0"))
  (set `CharacterMovementComponent.MaxWalkSpeed` (select `/Game/Game/Characters/Ennemy/AI/E_MovementSpeed` NewEnemyMovSpeed :`NewEnumerator0` (`self.Walking Speed`) :`NewEnumerator1` (`self.Running Speed`)) (`self.CharacterMovement`)))

(event `Attack`
  (`PrimitiveComponent.SetCollisionEnabled` (`self.Sphere`) "QueryAndPhysics")
  (`|PlayMontage` (`self.Mesh`) (`self.Attack Montage`)
    (:`OnCompleted`
      (`self.OnAttackEnd` true))
    (:`OnInterrupted`
      (`self.OnAttackEnd` false)))
  (`PrimitiveComponent.SetCollisionEnabled` (`self.Sphere`) "NoCollision")
  (set `self.HasHitOccured` false))

(event `self.Sphere.OnComponentBeginOverlap`
  (params (OverlappedComponent :type "PrimitiveComponent Object Reference") (OtherActor :type "Actor Object Reference") (OtherComp :type "PrimitiveComponent Object Reference") (OtherBodyIndex :type Integer) (bFromSweep :type Boolean) (SweepResult :type "HitResult Structure (by ref)"))
  (bind _asrpgcharacter (cast `RPGCharacter` OtherActor))
  (if (not (`self.HasHitOccured`))
    (set `self.HasHitOccured` true)
    (`GameplayStatics.ApplyDamage` _asrpgcharacter 3.0 null self)))

(fn `UserConstructionScript`)