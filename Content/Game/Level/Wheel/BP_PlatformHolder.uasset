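; BP_PlatformHolder is a holder actor that claims a random platform from a platform pool and carries it.
; On BeginPlay it claims immediately if WheelRef allows it, otherwise it binds to the wheel's readiness event.
; GetNewPlatform snaps a valid pool platform to the holder, keeping world scale, and stores it as HeldPlatform.
; A flag guards against double claims, and DestroyPlatform is an empty stub.
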(event `self.ReceiveBeginPlay`
  (if (`/Game/Game/Level/Wheel/BP_Wheel.CanGetPlatform` (`self.WheelRef`))
    (if (`self.Is holding platform`) :!label _label
      (`KismetSystemLibrary.PrintString` "DoubleClaiming platform")
      (else
        (`KismetSystemLibrary.PrintString` "Hello")
        (`self.GetNewPlatform`)
        (set `self.Is holding platform` true)))
    (else
      (add `/Game/Game/Level/Wheel/BP_Wheel.CanGetPlatforms` (`self.WheelRef`) (delegate `Platforms Ready`)))))

(event `Platforms Ready`
  (goto _label))

(fn `DestroyPlatform`)

(fn `GetNewPlatform`
  (bind _platform (`/Game/Game/Level/Wheel/Platforms/__PlatformPool.GetRandomPlatform` (`self.PlatformPoolRef`)))
  (if (`KismetSystemLibrary.IsValid` _platform)
    (`self.K2_AttachToActor` _platform self "None" "SnapToTarget" "SnapToTarget" "KeepWorld" true)
    (set `self.Held Platform` _platform)))

(fn `UserConstructionScript`)