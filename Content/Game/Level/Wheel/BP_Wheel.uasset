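; BP_Wheel is the rotating level wheel that carries platform holders, rolling each tick at the game state's WheelSpeed.
; On BeginPlay it builds zero-padded socket names from positions, rings and indices, then spawns and attaches a BP_PlatformHolder at each WheelMesh socket.
; Once both holders and the platform pool are ready, it calls CanGetPlatforms.
; It also starts the spin through BP_GameState, marked as a placeholder for a start menu.
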(event `self.ReceiveBeginPlay`
  (bind _outactors (`GameplayStatics.GetAllActorsOfClass` "/Game/Game/Level/Wheel/Platforms/__PlatformPool.__PlatformPool_C"))
  (bind _output_get (set `self.PoolRef` (`|GetArrayItem` _outactors)))
  (add `/Game/Game/Level/Wheel/Platforms/__PlatformPool.OnPoolReady` _output_get (delegate `PoolIsReady`))
  (`|ExecutionSequence`
    (:`then_0`
      (bind _generatednames (`self.GenerateSocketNames`))
      (if true
        (for _array_element _generatednames
          (bind _returnvalue (`|SpawnActorFromClass` "/Game/Game/Level/Wheel/BP_PlatformHolder.BP_PlatformHolder_C" (`self.GetTransform`) "Undefined" "MultiplyWithRoot" null (`self.PoolRef`) self null))
          (`KismetArrayLibrary.Array_Add` (`self.PlatformHolders`) _returnvalue)
          (bind _returnvalue_2 (`self.K2_AttachToComponent` _returnvalue (`self.WheelMesh`) _array_element "SnapToTarget" "SnapToTarget" "KeepWorld" true))
          (`SceneComponent.K2_SetRelativeRotation` (`/Game/Game/Level/Wheel/BP_PlatformHolder.DefaultSceneRoot` _returnvalue) (struct :`Roll` 90.0) false false))
        (`self.PlatformHoldersReady`)
        (else
          (`KismetSystemLibrary.PrintString` "INVALID REF"))))
    (:`then_1`
      (bind _asbp_game_state (cast `/Game/Game/Modes/BP_GameState` (`GameplayStatics.GetGameState`)))
      (bind _output_get_2 (set `self.Game State ref` _asbp_game_state))
      ; TODO: Replace with start menu or smth
      (`/Game/Game/Modes/BP_GameState.BeginWheelSpin` _output_get_2 5.0))))

(event `PoolIsReady`
  (`KismetSystemLibrary.PrintString` "PoolReady")
  (bind _output_get (set `self.PoolReady` true :!label _label))
  (if (and _output_get (stale `PlatformHoldersReady` _output_get)) :!label _label_2
    (`self.CanGetPlatforms`)
    (`KismetSystemLibrary.PrintString` "Calling Platforms")))

(event `PlatformHoldersReady`
  (`KismetSystemLibrary.PrintString` "HolderReady")
  (bind _output_get (set `self.HoldersReady` true))
  (if (`/Game/Game/Level/Wheel/Platforms/__PlatformPool.IsReady` (`self.PoolRef`))
    (goto _label)
    (else
      (goto _label_2))))

(event `self.ReceiveTick`
  (params (DeltaSeconds :type "Float (single-precision)"))
  (`self.K2_AddActorLocalRotation` (`KismetMathLibrary.MakeRotator` (* DeltaSeconds (`/Game/Game/Modes/BP_GameState.WheelSpeed` (`self.Game State ref`))))))

(fn `GenerateSocketNames`
  (returns (GeneratedNames :type "Array of Name"))
  (locals (Positions :type "Array of Text") (Rings :type "Array of Text") (GeneratedSocketNames :type "Array of Name"))
  (for _array_element (`local.Positions`)
    (for _array_element_2 (`local.Rings`)
      (for _index (range 1 31)
        (bind _string (`self.PaddedIntToString` _index))
        (`KismetArrayLibrary.Array_Add` (`local.GeneratedSocketNames`) (`KismetStringLibrary.Conv_StringToName` (`KismetTextLibrary.Conv_TextToString` (`|FormatText` "Wheel_{0}_{1}_{2}" _array_element _array_element_2 _string)))))))
  (return (`local.GeneratedSocketNames`)))

(fn `PaddedIntToString`
  (params (int :type Integer))
  (returns (string :type String))
  (locals (`Padding size` :type Integer :default 2) (asString :type String))
  (bind _output_get (set `local.asString` (`KismetStringLibrary.Conv_IntToString` int)))
  (for _ (range (`KismetStringLibrary.Len` _output_get) (+ (`local.Padding size`) 1))
    (set `local.asString` (`KismetStringLibrary.Concat_StrStr` "0" (`local.asString`))))
  (return (`local.asString`)))

(fn `UserConstructionScript`)