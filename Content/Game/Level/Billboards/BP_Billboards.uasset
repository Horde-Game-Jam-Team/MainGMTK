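; BP_Billboards is a level billboard that plays a randomly chosen video on a plane, in either vertical or horizontal orientation.
; The construction script scales the plane to match the IsVertical flag.
; On BeginPlay one random index picks the matching material, media player and video from that orientation's arrays, applies the material and opens the video source on the player.
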(event `self.ReceiveBeginPlay`
  (bind _randomselected (`self.RandomSelected`))
  (bind _randomselected_2 (`self.RandomSelected`))
  (set `self.RandomSelected` (`KismetMathLibrary.RandomIntegerInRange` 0 2))
  (`PrimitiveComponent.SetMaterial` (`self.Plane`) 0 (select `bool` (`self.isVertical`) :`false` (`|GetArrayItem` (`self.HorizontalMaterials`) (`self.RandomSelected`)) :`true` (`|GetArrayItem` (`self.VerticalMaterials`) (`self.RandomSelected`)) :!type "MaterialInterface Object Reference"))
  (`MediaPlayer.OpenSource` (select `bool` (`self.isVertical`) :`false` (`|GetArrayItem` (`self.MediaPlayerHorizontalRef`) _randomselected_2) :`true` (`|GetArrayItem` (`self.MediaPlayerVerticalRef`) _randomselected_2)) (select `bool` (`self.isVertical`) :`false` (`|GetArrayItem` (`self.HorizontalVideos`) _randomselected) :`true` (`|GetArrayItem` (`self.VerticalVideos`) _randomselected))))

(fn `UserConstructionScript`
  (bind _plane (`self.Plane`))
  (if (`self.isVertical`)
    (`SceneComponent.SetRelativeScale3D` _plane (1.0 1.5 1.0))
    (else
      (`SceneComponent.SetRelativeScale3D` _plane (1.7 1.0 1.0)))))