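; BP_Explosion is a short-lived explosion actor that damages enemies and removes itself one second after spawning.
; On BeginPlay it plays a random explosion sound, reports AI noise with the player character as instigator, and triggers a camera shake.
; The shake is centered on the player's location rather than the blast, while the noise uses the explosion's location.
; Any RPGEnemyBase that begins overlapping its Sphere component takes fixed damage.
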(event `self.ReceiveBeginPlay`
  (`self.Explode`)
  (`KismetSystemLibrary.Delay` 1.0)
  (`self.K2_DestroyActor`))

(event `self.Sphere.OnComponentBeginOverlap`
  (params (OverlappedComponent :type "PrimitiveComponent Object Reference") (OtherActor :type "Actor Object Reference") (OtherComp :type "PrimitiveComponent Object Reference") (OtherBodyIndex :type Integer) (bFromSweep :type Boolean) (SweepResult :type "HitResult Structure (by ref)"))
  (bind _asrpgenemy_base (cast `RPGEnemyBase` OtherActor))
  (`GameplayStatics.ApplyDamage` _asrpgenemy_base 3.0 null null "/Script/Engine.DamageType"))

(fn `Explode`
  (bind _returnvalue (`self.K2_GetActorLocation`))
  (`GameplayStatics.PlaySoundAtLocation` (`KismetArrayLibrary.Array_Random` (`self.Explosions`)) _returnvalue (struct) 1.0 1.0 0.0 null null null null)
  (bind _asbp_rpgcharacter (cast `/Game/Game/Characters/_Generic/BP_RPGCharacter` (`GameplayStatics.GetPlayerCharacter` 0)))
  (`self.MakeNoise` 1.0 _asbp_rpgcharacter _returnvalue)
  (`GameplayStatics.PlayWorldCameraShake` "/Game/Game/Characters/Player/LCS_CameraShake.LCS_CameraShake_C" (`self.K2_GetActorLocation` _asbp_rpgcharacter) 0.0 500.0))

(fn `UserConstructionScript`)