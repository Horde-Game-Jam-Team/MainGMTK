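; Actor component for the StickToFloor powerup that lets the first-person character treat much steeper slopes as walkable floor.
; On BeginPlay it casts its owner to BP_FirstPersonCharacter and caches that character's default walkable floor angle.
; SwitchOn raises the CharacterMovement walkable floor angle to vertical, and SwitchOff restores the cached default.
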(event `self.ReceiveBeginPlay`
  ; Begin Play
  (bind _asbp_first_person_character_ (cast `/Game/Game/Characters/Player/BP_FirstPersonCharacter` (`self.GetOwner`)))
  (bind _output_get (set `self.BPFirstPersonCharacter` _asbp_first_person_character_))
  (set `self.DefaultWalkableAngle` (`CharacterMovementComponent.K2_GetWalkableFloorAngle` (`Character.CharacterMovement` _output_get))))

(event `SwitchOn`
  ; Switch On PowerUp
  (`CharacterMovementComponent.SetWalkableFloorAngle` (`Character.CharacterMovement` (stale `self.ReceiveBeginPlay` _output_get)) 90.0))

(event `SwitchOff`
  ; Switch Off PowerUp
  (`CharacterMovementComponent.SetWalkableFloorAngle` (`Character.CharacterMovement` (stale `self.ReceiveBeginPlay` _output_get)) (`self.DefaultWalkableAngle`)))