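; BP_StickToFloor_PowerUp is a pickup that temporarily turns on the stick-to-floor ability when the first-person character walks through its box.
; Enable finds the player's AC_StickToFloor component, switches it on, and starts a timer that switches it off after PowerUpDuration.
; Re-entering clears any running timer first, so the duration restarts instead of stacking.
; The actor is not destroyed or hidden on pickup.
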(event `self.ReceiveBeginPlay`)

(event `Enable`
  (params (PlayerActor :type "Actor Object Reference"))
  (bind _poweruptimerhandle (`self.PowerUpTimerHandle`))
  ; Enabling Power-Up
  (if (`KismetSystemLibrary.K2_IsValidTimerHandle` _poweruptimerhandle)
    (`KismetSystemLibrary.K2_ClearAndInvalidateTimerHandle` _poweruptimerhandle))
  (bind _output_get (set `self.StickToFloorComponent` (`self.GetComponentByClass` PlayerActor "/Game/Game/Actors/Powerups/StickToFloor/AC_StickToFloor.AC_StickToFloor_C")))
  (`/Game/Game/Actors/Powerups/StickToFloor/AC_StickToFloor.SwitchOn` _output_get)
  (bind _returnvalue (`KismetSystemLibrary.K2_SetTimerDelegate` (delegate `Disable`) (`self.PowerUpDuration`)))
  (set `self.PowerUpTimerHandle` _returnvalue))

(event `Disable`
  ; Enabling Power-Up
  (`/Game/Game/Actors/Powerups/StickToFloor/AC_StickToFloor.SwitchOff` (stale `Enable` _output_get)))

(event `self.Box.OnComponentBeginOverlap`
  (params (OverlappedComponent :type "PrimitiveComponent Object Reference") (OtherActor :type "Actor Object Reference") (OtherComp :type "PrimitiveComponent Object Reference") (OtherBodyIndex :type Integer) (bFromSweep :type Boolean) (SweepResult :type "HitResult Structure (by ref)"))
  ; Take Power-Up when walking through it
  (if (== (`GameplayStatics.GetObjectClass` OtherActor) "/Game/Game/Characters/Player/BP_FirstPersonCharacter.BP_FirstPersonCharacter_C")
    (`self.Enable` OtherActor)))

(fn `UserConstructionScript`)