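; BP_ObjectSpawner is a portal actor that repeatedly throws objects toward the player.
; A looping timer set on BeginPlay spawns a BP_ObjectToSpawn at a random point within the portal mesh bounds, using the actor's initial rotation.
; Each object receives its start point and a randomized end point, which leads the player's target socket by a fixed distance along the last movement direction.
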(event `self.ReceiveBeginPlay`
  (set `self.InitialRotation` (`self.K2_GetActorRotation`))
  (`KismetSystemLibrary.K2_SetTimerDelegate` (delegate `ThrowObject`) (`self.SpawnTime`) true))

(event `ThrowObject`
  (bind _returnvalue (`GameplayStatics.GetPlayerCharacter` 0))
  (bind (_origin _boxextent) (`KismetSystemLibrary.GetComponentBounds` (`self.PortalMesh`)))
  (bind _output_get (set `self.RandomSpawnPoint` (`KismetMathLibrary.RandomPointInBoundingBox` _origin _boxextent)))
  (bind _returnvalue_2 (`|SpawnActorFromClass` "/Game/Game/Actors/PortalThrower/BP_ObjectToSpawn.BP_ObjectToSpawn_C" (`KismetMathLibrary.MakeTransform` _output_get (`self.InitialRotation`)) "Undefined" "MultiplyWithRoot" null self _output_get (`KismetMathLibrary.RandomPointInBoundingBox` (+ (`SceneComponent.GetSocketLocation` (`Character.Mesh` _returnvalue) (`self.CharacterTargetSocket`)) (* (`KismetMathLibrary.Normal` (`CharacterMovementComponent.GetLastUpdateVelocity` (`Character.CharacterMovement` _returnvalue))) 500.0)) (80.0 80.0 80.0)) null))
  (set `self.ThrownObject` _returnvalue_2))

(fn `UserConstructionScript`)