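; Physics prop thrown by a portal spawner that knocks back characters it strikes in flight.
; Construction picks a random mesh with a matching capsule, randomizes rotation and sets lifespan; BeginPlay launches it along a random arc to EndPos.
; The capsule's first overlap can launch listed character classes horizontally, weaker if falling, so the mesh avoids direct player collision.
; Hit, wake and sleep events track IsInAir, gating the knockback.
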(event `self.ReceiveBeginPlay`
  ; Ignore spawner when moving
  (`PrimitiveComponent.IgnoreActorWhenMoving` (`self.StaticMesh`) (`self.Spawner`) true)
  ; Projectile Arc Movement
  (bind _outlaunchvelocity (`GameplayStatics.SuggestProjectileVelocity_CustomArc` (`self.StartPos`) (`self.End Pos`) 0.0 (`KismetMathLibrary.RandomFloatInRange` 0.5 0.8)))
  (bind _output_get (set `self.LaunchVelocity` _outlaunchvelocity))
  (`PrimitiveComponent.SetPhysicsLinearVelocity` (`self.StaticMesh`) _output_get false "None"))

(event `self.Capsule.OnComponentBeginOverlap`
  (params (OverlappedComponent :type "PrimitiveComponent Object Reference") (OtherActor :type "Actor Object Reference") (OtherComp :type "PrimitiveComponent Object Reference") (OtherBodyIndex :type Integer) (bFromSweep :type Boolean) (SweepResult :type "HitResult Structure (by ref)"))
  (bind (_launchvelocity_x _launchvelocity_y) (`KismetMathLibrary.BreakVector` (`self.LaunchVelocity`)))
  (bind _returnvalue (* (`KismetMathLibrary.MakeVector` _launchvelocity_x _launchvelocity_y) (/ (`self.ImpulseStrength`) 100.0)))
  ; Apply impulse when capsule overlap characters, the static mesh itself will not collide with player directly avoiding rotation issue
  (`/Engine/EditorBlueprintResources/StandardMacros.DoOnce` false
    (:`Completed`
      (if (`KismetArrayLibrary.Array_Contains` (`self.CharactersWhoReceivesImpact`) (`GameplayStatics.GetObjectClass` OtherActor))
        ; Launch Character when overlap
        (bind _ascharacter (cast `Character` OtherActor))
        (if (`self.IsInAir`)
          (if (`NavMovementComponent.IsFalling` (`Character.CharacterMovement` _ascharacter))
            (`Character.LaunchCharacter` _ascharacter (/ _returnvalue 3.0) true false)
            (else
              (`Character.LaunchCharacter` _ascharacter _returnvalue true false))))))))

(event `self.StaticMesh.OnComponentHit`
  (params (HitComponent :type "PrimitiveComponent Object Reference") (OtherActor :type "Actor Object Reference") (OtherComp :type "PrimitiveComponent Object Reference") (NormalImpulse :type "Vector Structure") (Hit :type "HitResult Structure (by ref)"))
  (if (< (`KismetMathLibrary.VSize` (`SceneComponent.GetComponentVelocity` (`self.StaticMesh`))) 100.0)
    (set `self.IsInAir` false)
    (else
      (set `self.IsInAir` true))))

(event `self.StaticMesh.OnComponentWake`
  (params (WakingComponent :type "PrimitiveComponent Object Reference") (BoneName :type Name))
  (set `self.IsInAir` true))

(event `self.StaticMesh.OnComponentSleep`
  (params (SleepingComponent :type "PrimitiveComponent Object Reference") (BoneName :type Name))
  (set `self.IsInAir` false))

(fn `UserConstructionScript`
  (bind _meshstructure (`self.MeshStructure`))
  (`/Engine/EditorBlueprintResources/StandardMacros.DoOnce` false
    (:`Completed`
      (bind _output_get (set `self.RandomNumber` (`KismetMathLibrary.RandomIntegerInRange` 0 (- (`KismetArrayLibrary.Array_Length` _meshstructure) 1))))
      (`self.SetLifeSpan` (`self.InitialLifeSpan`))
      (bind (_mesh _defaultobjectrotation _capsulehalfsize _capsuleradius _capsulelocation _capsulerotation) (break `/Game/Game/Actors/PortalThrower/S_MeshData` (`|GetArrayItem` _meshstructure _output_get)))
      (`self.RandomMesh&Rotation` _mesh _defaultobjectrotation _capsulehalfsize _capsuleradius _capsulelocation _capsulerotation))))